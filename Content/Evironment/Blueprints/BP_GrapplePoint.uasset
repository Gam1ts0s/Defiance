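; BP_GrapplePoint is a world grapple point that shows an on-screen indicator of how close the player is to grapple range.
; Activate and deactivate events pass player and range data to the grapple logic and toggle the widget's visibility.
; While active, Tick maps player distance between detection and interact ranges onto a progress bar, turning it from grey to green within interact range.
; BeginPlay caches the widget and LandingZone's relative location; OnInteract is empty.
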(event `self.ReceiveBeginPlay`
  (bind _returnvalue_location (`KismetMathLibrary.BreakTransform` (`SceneComponent.GetRelativeTransform` (`self.LandingZone`))))
  (bind _asgrapple_point (cast `/Game/UI/GrapplePoint` (`WidgetComponent.GetUserWidgetObject` (`self.GrappleHookWidget`))))
  (set `self.GrapplePointWidget` _asgrapple_point)
  (set `self.LandingLocation` _returnvalue_location))

(event `self.ReceiveTick`
  (params (DeltaSeconds :type "Float (single-precision)"))
  (if (`self.bIsActive`)
    (`self.UpdateWidget`)))

(event `self.OnActivate`
  (params (PlayerPawnRef :type "Pawn Object Reference") (InteractRange :type "Float (single-precision)") (DetectionRange :type "Float (single-precision)"))
  (`self.ActivateGrapplePoint` PlayerPawnRef InteractRange DetectionRange)
  (if (`self.bIsActive`)
    (`SceneComponent.SetVisibility` (`self.GrappleHookWidget`) true false)))

(event `self.OnDeactivate`
  (`self.DeactivateGrapplePoint`)
  (`SceneComponent.SetVisibility` (`self.GrappleHookWidget`) false false))

(event `self.OnInteract`)

(fn `UpdateWidget`
  (bind _returnvalue (`KismetMathLibrary.MapRangeClamped` (`self.DistanceToPlayer`) (`self.PlayerInteractRange`) (`self.PlayerDetectionRange`) 0.8 0.2))
  (bind _progressbar (`/Game/UI/GrapplePoint.ProgressBar` (`self.GrapplePointWidget`)))
  (`ProgressBar.SetPercent` _progressbar _returnvalue)
  (`ProgressBar.SetFillColorAndOpacity` _progressbar (`KismetMathLibrary.SelectColor` (struct :`R` 0.184336 :`G` 0.630208 :`B` 0.160834 :`A` 0.7) (struct :`R` 0.571125 :`G` 0.571125 :`B` 0.571125 :`A` 0.701961) (== _returnvalue 0.8))))

(fn `UserConstructionScript`)